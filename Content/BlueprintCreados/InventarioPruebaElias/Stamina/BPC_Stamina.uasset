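; Stamina component (BPC_Stamina) that spends and regenerates its owner's stamina.
; DisminuirStamina subtracts a clamped cost, requests regeneration and fires UpdateStamina with the new value.
; A looping timer adds RegeneracionTick per interval, firing the same update, and is cleared by function name on finding stamina at maximum.
; The Regenera flag gates timer setup but is only ever set false here.
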(event Custom|RegeneracionDeStamina
  (if (not (Variables|Default|GetRegenera?))
    (Utilities|Time|SetTimerbyEvent (delegate Custom|RegenerarStamina) (Variables|Default|GetTiempoRegeneracionStamina) true)))

(event Custom|RegenerarStamina
  (if (!= (Variables|Default|GetStamina) (Variables|Default|GetStaminaMaxima))
    (bind _output_get (Variables|Default|SetStamina (Math|Float|Clamp(Float) (+ (Variables|Default|GetRegeneracionTick) (Variables|Default|GetStamina)) 0.0 (Variables|Default|GetStaminaMaxima))))
    (Default|CallUpdateStamina _output_get)
    (else
      (Variables|Default|SetRegenera? false)
      (Utilities|Time|ClearTimerbyFunctionName 0 "RegenerarStamina"))))

(event EventBeginPlay)

(event EventTick
  (params (DeltaSeconds :type Float%20%28single-precision%29)))

(fn DisminuirStamina
  (params (StaminaGastado :type Float%20%28double-precision%29))
  (bind _output_get (Variables|Default|SetStamina (Math|Float|Clamp(Float) (- (Variables|Default|GetStamina) StaminaGastado) 0.0 (Variables|Default|GetStaminaMaxima))))
  (CallFunction|RegeneracionDeStamina)
  (Default|CallUpdateStamina _output_get))