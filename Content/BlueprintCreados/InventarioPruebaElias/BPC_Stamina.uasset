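; Stamina component that handles spending and timed regeneration of a clamped stamina value.
; DisminuirStamina subtracts the cost, calls RegeneracionDeStamina to start a looping RegenerarStamina timer when Regenera is false, and broadcasts the new value through CallUpdateStamina.
; Each timer tick adds RegeneracionTick and broadcasts until Stamina reaches StaminaMaxima, then clears the timer by function name.
; Regenera guards the timer start, but this graph only ever sets it to false.
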(event Custom|RegeneracionDeStamina
  (if (not (Variables|Default|GetRegenera?))
    (Utilities|Time|SetTimerbyEvent (delegate Custom|RegenerarStamina) (Variables|Tiempo|GetTiempoRegeneracionStamina) true)))

(event Custom|RegenerarStamina
  (if (!= (Variables|ValoresDeStamina|GetStamina) (Variables|ValoresDeStamina|GetStaminaMaxima))
    (bind _output_get (Variables|ValoresDeStamina|SetStamina (Math|Float|Clamp(Float) (+ (Variables|Tiempo|GetRegeneracionTick) (Variables|ValoresDeStamina|GetStamina)) 0.0 (Variables|ValoresDeStamina|GetStaminaMaxima))))
    (Default|CallCallUpdateStamina _output_get)
    (else
      (Variables|Default|SetRegenera? false)
      (Utilities|Time|ClearTimerbyFunctionName 0 "RegenerarStamina"))))

(event EventBeginPlay)

(event EventTick
  (params (DeltaSeconds :type Float%20%28single-precision%29)))

(fn DisminuirStamina
  (params (StaminaGastado :type Float%20%28double-precision%29))
  (bind _output_get (Variables|ValoresDeStamina|SetStamina (Math|Float|Clamp(Float) (- (Variables|ValoresDeStamina|GetStamina) StaminaGastado) 0.0 (Variables|ValoresDeStamina|GetStaminaMaxima))))
  (CallFunction|RegeneracionDeStamina)
  (Default|CallCallUpdateStamina _output_get))