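; Inventory Blueprint that holds ten item slots and lets the player pick up world items.
; BeginPlay creates WB_Inventario and loads it from the Items array; I toggles the widget and input mode.
; E sphere-traces around the player for a BP_ItemInventario, placing it in the first slot that is empty or can stack it up to 64.
; A successful pickup refreshes the widget and destroys the world actor.
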(event EventBeginPlay
  (bind _returnvalue (UserInterface|CreateWidget "/Game/BlueprintCreados/InventarioPruebaElias/Widget/WB_Inventario.WB_Inventario_C"))
  (Variables|Default|SetInventariodelWidget _returnvalue)
  (Utilities|Array|Resize (Variables|Default|GetItems) 10)
  (Default|CargarInventario (Variables|Default|GetInventariodelWidget) self))

(event EventTick
  (params (DeltaSeconds :type Float%20%28single-precision%29)))

(event Input|KeyboardEvents|E
  (params (Key :type Key%20Structure :default "None"))
  (bind _returnvalue (Game|GetPlayerCharacter 0))
  (bind _returnvalue_2 (Transformation|GetActorLocation _returnvalue))
  (bind _returnvalue_3 (- _returnvalue_2 "0.000000,0.000000,10.000000"))
  (:Pressed
    (bind _outhit (Collision|SphereTraceByChannel _returnvalue_3 _returnvalue_3 1.2e+02 "TraceTypeQuery1" false 0 "ForDuration"))
    (bind _asbp_item_inventario (Utilities|Casting|CastToBP_ItemInventario (.HitActor (Collision|BreakHitResult _outhit))))
    (for (_array_element _array_index) (Variables|Default|GetItems)
      (Utilities|IsValid _asbp_item_inventario
        (:Is%20Valid
          (if (Math|Boolean|ANDBoolean (Utilities|Enum|Equal(Enum) (.Nombre (Utilities|Struct|BreakST_Item _array_element)) (.Nombre (Utilities|Struct|BreakST_Item (Variables|/Game/BlueprintCreados/InventarioPruebaElias/Blueprint/BP_ItemInventario.BP_ItemInventario_C|GetItem _asbp_item_inventario)))) (.Stackable (Utilities|Struct|BreakST_Item (Variables|/Game/BlueprintCreados/InventarioPruebaElias/Blueprint/BP_ItemInventario.BP_ItemInventario_C|GetItem _asbp_item_inventario))) (<= (+ (.Cantidad (Utilities|Struct|BreakST_Item _array_element)) (.Cantidad (Utilities|Struct|BreakST_Item (Variables|/Game/BlueprintCreados/InventarioPruebaElias/Blueprint/BP_ItemInventario.BP_ItemInventario_C|GetItem _asbp_item_inventario)))) 64))
            (Utilities|Array|SetArrayElem (Variables|Default|GetItems) _array_index (Utilities|Struct|MakeST_Item (.nombre (Variables|/Game/BlueprintCreados/InventarioPruebaElias/Blueprint/BP_ItemInventario.BP_ItemInventario_C|GetItem _asbp_item_inventario)) (+ (.Cantidad (Utilities|Struct|BreakST_Item _array_element)) (.Cantidad (Utilities|Struct|BreakST_Item (Variables|/Game/BlueprintCreados/InventarioPruebaElias/Blueprint/BP_ItemInventario.BP_ItemInventario_C|GetItem _asbp_item_inventario)))) (.mesh (Variables|/Game/BlueprintCreados/InventarioPruebaElias/Blueprint/BP_ItemInventario.BP_ItemInventario_C|GetItem _asbp_item_inventario)) (.stackable (Variables|/Game/BlueprintCreados/InventarioPruebaElias/Blueprint/BP_ItemInventario.BP_ItemInventario_C|GetItem _asbp_item_inventario)) (.thumnail (Variables|/Game/BlueprintCreados/InventarioPruebaElias/Blueprint/BP_ItemInventario.BP_ItemInventario_C|GetItem _asbp_item_inventario))))
            (Default|CargarInventario (Variables|Default|GetInventariodelWidget) self :!label _label)
            (Actor|DestroyActor _asbp_item_inventario)
            (elif (== (.Cantidad (Utilities|Struct|BreakST_Item _array_element)) 0)
              (Utilities|Array|SetArrayElem (Variables|Default|GetItems) _array_index (Variables|/Game/BlueprintCreados/InventarioPruebaElias/Blueprint/BP_ItemInventario.BP_ItemInventario_C|GetItem _asbp_item_inventario))
              (goto _label))))))))

(event Input|KeyboardEvents|1
  (params (Key :type Key%20Structure :default "None")))

(event Input|KeyboardEvents|I
  (params (Key :type Key%20Structure :default "None"))
  (bind _returnvalue (Game|GetPlayerController 0))
  (bind _returnvalue_2 (Game|GetPlayerController 0))
  (bind _inventariodelwidget (Variables|Default|GetInventariodelWidget))
  (:Pressed
    (if (Widget|IsVisible (Variables|Default|GetInventariodelWidget))
      (Widget|RemovefromParent _inventariodelwidget)
      (Variables|/Script/Engine.PlayerController|SetbShowMouseCursor _returnvalue true)
      (Input|SetInputModeGameOnly _returnvalue false)
      (else
        (Variables|/Script/Engine.PlayerController|SetbShowMouseCursor _returnvalue_2 true)
        (Input|SetInputModeGameandUI _returnvalue_2 0 "DoNotLock" true false)
        (UserInterface|Viewport|AddtoViewport _inventariodelwidget 0)))))