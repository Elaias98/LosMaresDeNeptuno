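; BP_Cofre is a chest that hands out inventory items when any actor overlaps its box.
; While SpawneoA is set and the count is below its maximum, each overlap spawns an apple BP_ItemInventario at that actor's transform and increments the count.
; SpawneoA re-arms immediately, while SpawneoB gates a one-time sword spawn within the same branch.
; Debug prints report the spawn condition and sword name.
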(event OnComponentBeginOverlap(Box)
  (params (OverlappedComponent :type Primitive%20Component%20Object%20Reference) (OtherActor :type Actor%20Object%20Reference) (OtherComp :type Primitive%20Component%20Object%20Reference) (OtherBodyIndex :type Integer) (bFromSweep :type Boolean) (SweepResult :type Hit%20Result%20Structure%20%28by%20ref%29))
  (Development|PrintString (Utilities|String|ToString(Boolean) (and (Variables|Default|GetSpawneoA?) (< (Variables|Default|GetCantidadActual) (Variables|Default|GetCantidadMax)))))
  (if (and (Variables|Default|GetSpawneoA?) (< (Variables|Default|GetCantidadActual) (Variables|Default|GetCantidadMax)))
    (Game|SpawnActorfromClass "/Game/BlueprintCreados/InventarioPruebaElias/Blueprint/BP_ItemInventario.BP_ItemInventario_C" (Transformation|GetActorTransform OtherActor) "Undefined" "MultiplyWithRoot" 0 (Utilities|Struct|MakeST_Item "Manzana" 1 "/Game/BlueprintCreados/InventarioPruebaElias/ModeloPrueba/SM_Apple.SM_Apple" true "/Game/BlueprintCreados/InventarioPruebaElias/ModeloPrueba/TApplethumbnail.TApplethumbnail") 0)
    (Variables|Default|SetSpawneoA? false)
    (Variables|Default|SetCantidadActual (+ (Variables|Default|GetCantidadActual) 1))
    (Variables|Default|SetSpawneoA? true)
    (if (Variables|Default|GetSpawneoB?)
      (bind _returnvalue (Game|SpawnActorfromClass "/Game/BlueprintCreados/InventarioPruebaElias/Blueprint/BP_ItemInventario.BP_ItemInventario_C" (Transformation|GetActorTransform OtherActor) "Undefined" "MultiplyWithRoot" 0 (Utilities|Struct|MakeST_Item "Espada" 1 "/Game/BlueprintCreados/InventarioPruebaElias/ModeloPrueba/SM_DIamondsword.SM_DIamondsword" true "/Game/BlueprintCreados/InventarioPruebaElias/ModeloPrueba/T_Minecraftswordthumbnail.T_Minecraftswordthumbnail") 0))
      (Development|PrintString (Utilities|GetDisplayName _returnvalue))
      (Variables|Default|SetSpawneoB? false))))

(event EventBeginPlay)

(event Collision|EventActorBeginOverlap
  (params (OtherActor :type Actor%20Object%20Reference)))

(event EventTick
  (params (DeltaSeconds :type Float%20%28single-precision%29)))

(fn ConstructionScript)