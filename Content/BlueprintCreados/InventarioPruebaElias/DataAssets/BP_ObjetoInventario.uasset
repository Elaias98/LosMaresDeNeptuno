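; Inventory pickup actor that hands its item to the player on contact.
; The construction script sets the static mesh from the assigned ItemInfo, when one is set.
; When a BP_ThirdPersonCharacter overlaps the sphere, it passes ItemInfo to that character's RecogerInventario and prints the item's name.
; The actor does not destroy or hide itself after the overlap.
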(event OnComponentBeginOverlap(Sphere)
  (params (OverlappedComponent :type Primitive%20Component%20Object%20Reference) (OtherActor :type Actor%20Object%20Reference) (OtherComp :type Primitive%20Component%20Object%20Reference) (OtherBodyIndex :type Integer) (bFromSweep :type Boolean) (SweepResult :type Hit%20Result%20Structure%20%28by%20ref%29))
  (bind _iteminfo (Variables|Inventario|GetItemInfo))
  (bind _asbp_third_person_character (Utilities|Casting|CastToBP_ThirdPersonCharacter OtherActor))
  (Default|RecogerInventario _asbp_third_person_character _iteminfo)
  (Development|PrintString (Variables|/Game/BlueprintCreados/InventarioPruebaElias/DataAssets/DA_ItemInventario.DA_ItemInventario_C|GetNombre _iteminfo)))

(event EventBeginPlay)

(event Collision|EventActorBeginOverlap
  (params (OtherActor :type Actor%20Object%20Reference)))

(event EventTick
  (params (DeltaSeconds :type Float%20%28single-precision%29)))

(fn ConstructionScript
  (if (!= (Variables|Inventario|GetItemInfo) 0)
    (Components|StaticMesh|SetStaticMesh (Variables|Default|GetStaticMesh) (Variables|/Game/BlueprintCreados/InventarioPruebaElias/DataAssets/DA_ItemInventario.DA_ItemInventario_C|GetMesh (Variables|Inventario|GetItemInfo)))))