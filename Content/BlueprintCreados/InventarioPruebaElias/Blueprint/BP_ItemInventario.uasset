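; BP_ItemInventario is a world actor for an inventory item, showing the item's mesh as a physics object.
; On BeginPlay it waits briefly, then applies the mesh from its Item data to the StaticMesh component and enables physics simulation.
; The construction script's copy of this setup is disconnected, so the mesh is assigned only at runtime, and the file contains no pickup logic.
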(event EventBeginPlay
  (Utilities|FlowControl|Delay 1.0)
  (Components|StaticMesh|SetStaticMesh (Variables|Default|GetStaticMesh) (.mesh (Variables|Default|GetItem)))
  (Physics|SetSimulatePhysics (Variables|Default|GetStaticMesh) true))

(event Collision|EventActorBeginOverlap
  (params (OtherActor :type Actor%20Object%20Reference)))

(event EventTick
  (params (DeltaSeconds :type Float%20%28single-precision%29)))

(fn ConstructionScript)